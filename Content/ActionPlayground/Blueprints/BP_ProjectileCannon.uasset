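; BP_ProjectileCannon is a cannon actor that repeatedly fires magic projectiles in the action playground.
; A looping half-second timer set on BeginPlay spawns a BP_MagicProjectile at the actor's transform.
; Each Tick rotates the Arrow component in world space to face the first player's pawn, while the spawn reads the actor transform rather than the Arrow's.
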(event Custom|SpawnActor
  (Game|SpawnActorfromClass "/Game/ActionPlayground/Blueprints/BP_MagicProjectile.BP_MagicProjectile_C" (Transformation|GetActorTransform) "Undefined" 0 0))

(event EventBeginPlay
  (Utilities|Time|SetTimerbyEvent (delegate Custom|SpawnActor) 0.5 true))

(event EventTick
  (params (DeltaSeconds :type Float%20%28single-precision%29))
  (Transformation|SetWorldRotation (Variables|Default|GetArrow) (Math|Rotator|MakeRotfromX (- (Transformation|GetActorLocation (Game|Player|GetPlayerPawn 0)) (Transformation|GetActorLocation))) false false))

(fn ConstructionScript)